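; BP_Door is a double sliding door driven by a set of linked buttons, open only while all are active.
; BeginPlay caches closed positions, derives open ones by offsetting each leaf along local X, and binds to each button's pressed-changed event.
; CheckButtons plays DoorTimeline forward or in reverse to lerp both leaves.
; An IsOpen flag guards opening, but nothing clears it and closing is unguarded.
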(event `self.ReceiveBeginPlay`
  (bind _output_get (set `self.LeftClosedLocation` (`SceneComponent.RelativeLocation` (`self.LeftDoor`))))
  (bind _output_get_2 (set `self.RightClosedLocation` (`SceneComponent.RelativeLocation` (`self.RightDoor`))))
  (set `self.RightOpenLocation` (+ _output_get_2 (150.0 0.0 0.0)))
  (set `self.LeftOpenLocation` (+ _output_get (-150.0 0.0 0.0)))
  (for _array_element (`self.Buttons`)
    (add `/Game/00_Examen_UNIR/Blueprints/BP_FloorButton.OnPressedChanged` _array_element (`|CreateDelegate` :!event `CheckButtons`))))

(event `CheckButtons`
  (set `self.AllPressed` true)
  (for _array_element (`self.Buttons`)
    (if (not (`/Game/00_Examen_UNIR/Blueprints/BP_FloorButton.IsActive` _array_element))
      (set `self.AllPressed` false)))
  (if (`self.AllPressed`)
    (`self.OpenDoor`)
    (else
      (`self.CloseDoor`))))

(event `OpenDoor`
  (if (not (`self.IsOpen`))
    (bind (_direction _alpha) (`Timeline|DoorTimeline` :!via `PlayFromStart` :!label _label)
      (:`Update`
        (set `self.IsOpen` true)
        (`SceneComponent.K2_SetRelativeLocation` (`self.LeftDoor`) (`KismetMathLibrary.VLerp` (`self.LeftClosedLocation`) (`self.LeftOpenLocation`) _alpha) false false)
        (`SceneComponent.K2_SetRelativeLocation` (`self.RightDoor`) (`KismetMathLibrary.VLerp` (`self.RightClosedLocation`) (`self.RightOpenLocation`) _alpha) false false)))))

(event `CloseDoor`
  (goto _label :!via `ReverseFromEnd`))

(fn `UserConstructionScript`)