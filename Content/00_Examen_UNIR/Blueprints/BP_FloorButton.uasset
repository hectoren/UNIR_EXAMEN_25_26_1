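; BP_FloorButton is a floor button that toggles an active state and shows it through an emissive material.
; ToggleButton flips IsActive, swaps the LightButton material to match, then fires OnPressedChanged to announce the change.
; The Trigger begin and end overlap events only cast to BP_FirstPersonCharacter; neither calls ToggleButton or does anything further.
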(event `self.Trigger.OnComponentBeginOverlap`
  (params (OverlappedComponent :type "PrimitiveComponent Object Reference") (OtherActor :type "Actor Object Reference") (OtherComp :type "PrimitiveComponent Object Reference") (OtherBodyIndex :type Integer) (bFromSweep :type Boolean) (SweepResult :type "HitResult Structure (by ref)"))
  (cast `/Game/FirstPerson/Blueprints/BP_FirstPersonCharacter` OtherActor))

(event `self.Trigger.OnComponentEndOverlap`
  (params (OverlappedComponent :type "PrimitiveComponent Object Reference") (OtherActor :type "Actor Object Reference") (OtherComp :type "PrimitiveComponent Object Reference") (OtherBodyIndex :type Integer))
  (cast `/Game/FirstPerson/Blueprints/BP_FirstPersonCharacter` OtherActor))

(fn `ToggleButton`
  (bind _lightbutton (`self.LightButton`))
  (set `self.IsActive` (not (`self.IsActive`)))
  (if (`self.IsActive`)
    (`PrimitiveComponent.SetMaterial` _lightbutton 0 "/Game/LowPolyAssets/Materials/M_Emission_Platform.M_Emission_Platform")
    (else
      (`PrimitiveComponent.SetMaterial` _lightbutton 0 "/Game/LowPolyAssets/Materials/M_Emission.M_Emission")))
  (`self.OnPressedChanged`))

(fn `UserConstructionScript`)